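; Spawner actor that fills the level with a row of CubeWithSpotMaterial actors on BeginPlay, each with a randomized material look.
; A loop spawns the cubes at evenly stepped world-space offsets from its StaticMesh, copying that mesh's rotation and scale and ignoring collisions.
; Each cube then receives random values for two X/Y pairs of scalar material parameters, varying the material per instance.
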(event EventBeginPlay
  (bind _staticmesh (Variables|Default|GetStaticMesh))
  (bind _returnvalue (Transformation|GetWorldTransform _staticmesh))
  (for _index (range 1 20)
    (bind _returnvalue_2 (Game|SpawnActorfromClass "/Game/Blueprints/CubeWithSpotMaterial.CubeWithSpotMaterial_C" (Math|Transform|MakeTransform (+ (.location _returnvalue) (* (Math|Vector|MakeVector 5e+02 1e+02 0.0) _index)) (.rotation _returnvalue) (.scale _returnvalue)) "AlwaysSpawn" 0 0))
    (Rendering|Material|SetScalarParameterValueonMaterials (Variables|/Game/Blueprints/CubeWithSpotMaterial.CubeWithSpotMaterial_C|GetCube _returnvalue_2) "X1" (Math|Random|RandomFloat))
    (Rendering|Material|SetScalarParameterValueonMaterials (Variables|/Game/Blueprints/CubeWithSpotMaterial.CubeWithSpotMaterial_C|GetCube _returnvalue_2) "Y1" (Math|Random|RandomFloat))
    (Rendering|Material|SetScalarParameterValueonMaterials (Variables|/Game/Blueprints/CubeWithSpotMaterial.CubeWithSpotMaterial_C|GetCube _returnvalue_2) "X2" (Math|Random|RandomFloat))
    (Rendering|Material|SetScalarParameterValueonMaterials (Variables|/Game/Blueprints/CubeWithSpotMaterial.CubeWithSpotMaterial_C|GetCube _returnvalue_2) "Y2" (Math|Random|RandomFloat))))

(event Collision|EventActorBeginOverlap
  (params (OtherActor :type Actor%20Object%20Reference)))

(event EventTick
  (params (DeltaSeconds :type Float%20%28single-precision%29)))

(fn ConstructionScript)